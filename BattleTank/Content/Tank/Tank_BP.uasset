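; Player-controllable tank Blueprint that assembles the vehicle from parts and provides an orbiting aim camera.
; The construction script snaps the turret and both tracks to sockets on the Tank body, and the barrel to the turret.
; AimAzimuth and AimElevation axis inputs add frame-time-scaled local yaw and pitch to the SpringArm, leaving turret and barrel unrotated.
; Driving and firing are absent, and the event graph holds only empty stubs.
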(event OnComponentBeginOverlap(Tank)
  (params (OverlappedComponent :type Primitive%20Component%20Object%20Reference) (OtherActor :type Actor%20Object%20Reference) (OtherComp :type Primitive%20Component%20Object%20Reference) (OtherBodyIndex :type Integer) (bFromSweep :type Boolean) (SweepResult :type Hit%20Result%20Structure%20%28by%20ref%29)))

(event EventBeginPlay)

(event Collision|EventActorBeginOverlap
  (params (OtherActor :type Actor%20Object%20Reference)))

(event EventTick
  (params (DeltaSeconds :type Float%20%28single-precision%29)))

(event Input|AxisEvents|InputAxisAimAzimuth
  (params (AxisValue :type Float%20%28single-precision%29))
  ;[1 1 1] Camera Input Binding
  (Transformation|AddLocalRotation (Variables|Default|GetSpringArm) (Math|Rotator|MakeRotator 0.0 0.0 (* AxisValue (Utilities|Time|GetWorldDeltaSeconds) 1e+02)) false false))

(event Input|AxisEvents|InputAxisAimElevation
  (params (AxisValue :type Float%20%28single-precision%29))
  ;[1 1 1] Camera Input Binding
  (Transformation|AddLocalRotation (Variables|Default|GetSpringArm) (Math|Rotator|MakeRotator 0.0 (* AxisValue (Utilities|Time|GetWorldDeltaSeconds) 1e+02) 0.0) false false))

(fn ConstructionScript
  (Transformation|AttachComponentToComponent (Variables|Default|GetBarrel) (Variables|Default|GetTurret) "None" "SnapToTarget" "KeepRelative" "KeepRelative" true)
  (Transformation|AttachComponentToComponent (Variables|Default|GetTurret) (Variables|Default|GetTank) "Turret" "SnapToTarget" "KeepRelative" "KeepRelative" true)
  (Transformation|AttachComponentToComponent (Variables|Default|GetLeft%20Track) (Variables|Default|GetTank) "Tread_Left" "SnapToTarget" "KeepRelative" "KeepRelative" true)
  (Transformation|AttachComponentToComponent (Variables|Default|GetRight%20Track) (Variables|Default|GetTank) "Tread_Right" "SnapToTarget" "KeepRelative" "KeepRelative" true))